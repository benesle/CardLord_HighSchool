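; Lamp actor with a point light that can optionally flicker during play.
; The construction script applies the on/off state, scaled intensity and attenuation radius to the light.
; When Flickering is set, BeginPlay runs an endless loop that toggles light visibility after short random delays.
; Each loop also sets the same lit material on LampA, so the mesh material does not follow the on/off state.
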(event `self.ReceiveBeginPlay`
  (if (`self.Flickering`)
    (`SceneComponent.SetVisibility` (`self.PointLight`) (`self.LightOn`) false :!label _label)
    (`KismetSystemLibrary.Delay` (`KismetMathLibrary.RandomFloatInRange` 0.05 0.3))
    (set `self.LightOn` (not (`self.LightOn`)))
    (`PrimitiveComponent.SetMaterial` (`self.Lamp_A`) 0 "/Game/Assets/Materials/Lamp_light_Inst.Lamp_light_Inst")
    (goto _label)))

(fn `UserConstructionScript`
  (locals (`Actual intensity` :type "Float (double-precision)" :default 1000.0))
  (bind _pointlight (`self.PointLight`))
  (`SceneComponent.SetVisibility` _pointlight (`self.LightOn`) true)
  (`LightComponent.SetIntensity` _pointlight (* (`local.Actual intensity`) (`self.LightIntensity`)))
  (`LocalLightComponent.SetAttenuationRadius` _pointlight (`self.Attenuation radius`)))