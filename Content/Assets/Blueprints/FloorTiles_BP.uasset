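; Procedural floor slab actor that builds a tiled block from Width, Length and Thickness in its construction script.
; Instanced static mesh components lay out the top tile grid, optional stacked side rows rotated per North, East, South and West edge, and an optional flipped underside.
; A slightly shrunk Cube1 is scaled and centred to fill the interior, shown only when InsideBox is set.
; The event graph holds no runtime logic.
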(fn `UserConstructionScript`
  (locals (LocalTileSize :type Integer :default 100) (LocalSideThickness :type Integer :default -5) (LocalWidthIndex :type Integer) (LocalLengthIndex :type Integer) (LocalThicknessIndex :type Integer) (LocalTotalWidth :type Integer) (LocalTotalLength :type Integer) (LocalTotalThickness :type Integer))
  (bind _cube1 (`self.Cube1`))
  (bind _localtilesize (`local.LocalTileSize`))
  (bind _localtilesize_2 (`local.LocalTileSize`))
  (set `local.LocalTotalThickness` (* (`self.Thickness`) (`local.LocalSideThickness`)))
  (set `local.LocalTotalWidth` (* (`self.Width`) (`local.LocalTileSize`)))
  (set `local.LocalTotalLength` (* (`self.Length`) (`local.LocalTileSize`)))
  (bind _returnvalue (`AddComponent|NODE_AddInstancedStaticMeshComponent-2`))
  (for _index (range (`self.Width`))
    (set `local.LocalWidthIndex` _index)
    (for _index_2 (range (`self.Length`))
      (bind _output_get (set `local.LocalLengthIndex` _index_2))
      (`InstancedStaticMeshComponent.AddInstance` _returnvalue (`KismetMathLibrary.MakeTransform` (`KismetMathLibrary.MakeVector` (`KismetMathLibrary.Conv_IntToDouble` (* _output_get _localtilesize_2)) (`KismetMathLibrary.Conv_IntToDouble` (* _localtilesize_2 (`local.LocalWidthIndex`))))))))
  (if (`self.South`)
    ;[1 1 1] South
    (bind _returnvalue_2 (`AddComponent|NODE_AddInstancedStaticMeshComponent-4` :`RelativeTransform` (`KismetMathLibrary.MakeTransform` (0.0 0.0 0.0))))
    (for _index_3 (range (`self.Thickness`))
      (set `local.LocalThicknessIndex` _index_3)
      (for _index_4 (range (`self.Width`))
        (set `local.LocalWidthIndex` _index_4)
        (`InstancedStaticMeshComponent.AddInstance` _returnvalue_2 (`KismetMathLibrary.MakeTransform` (`KismetMathLibrary.MakeVector` 0.0 (`KismetMathLibrary.Conv_IntToDouble` (* (`local.LocalWidthIndex`) (`local.LocalTileSize`))) (`KismetMathLibrary.Conv_IntToDouble` (* (`local.LocalSideThickness`) (`local.LocalThicknessIndex`)))))))))
  (if (`self.East`)
    ;[1 1 1] East
    (bind _returnvalue_3 (`AddComponent|NODE_AddInstancedStaticMeshComponent-6` :`RelativeTransform` (`KismetMathLibrary.MakeTransform` (`KismetMathLibrary.MakeVector` 0.0 (`KismetMathLibrary.Conv_IntToDouble` (`local.LocalTotalWidth`))) (struct :`Yaw` -90.0))))
    (for _index_5 (range (`self.Thickness`))
      (set `local.LocalThicknessIndex` _index_5)
      (for _index_6 (range (`self.Length`))
        (set `local.LocalLengthIndex` _index_6)
        (`InstancedStaticMeshComponent.AddInstance` _returnvalue_3 (`KismetMathLibrary.MakeTransform` (`KismetMathLibrary.MakeVector` 0.0 (`KismetMathLibrary.Conv_IntToDouble` (* (`local.LocalLengthIndex`) (`local.LocalTileSize`))) (`KismetMathLibrary.Conv_IntToDouble` (* (`local.LocalSideThickness`) (`local.LocalThicknessIndex`)))))))))
  (if (`self.North`)
    ;[1 1 1] North
    (bind _returnvalue_4 (`AddComponent|NODE_AddInstancedStaticMeshComponent-7` :`RelativeTransform` (`KismetMathLibrary.MakeTransform` (`KismetMathLibrary.MakeVector` (`KismetMathLibrary.Conv_IntToDouble` (`local.LocalTotalLength`)) (`KismetMathLibrary.Conv_IntToDouble` (`local.LocalTotalWidth`))) (struct :`Yaw` -180.0))))
    (for _index_7 (range (`self.Thickness`))
      (set `local.LocalThicknessIndex` _index_7)
      (for _index_8 (range (`self.Width`))
        (set `local.LocalWidthIndex` _index_8)
        (`InstancedStaticMeshComponent.AddInstance` _returnvalue_4 (`KismetMathLibrary.MakeTransform` (`KismetMathLibrary.MakeVector` 0.0 (`KismetMathLibrary.Conv_IntToDouble` (* (`local.LocalWidthIndex`) (`local.LocalTileSize`))) (`KismetMathLibrary.Conv_IntToDouble` (* (`local.LocalSideThickness`) (`local.LocalThicknessIndex`)))))))))
  (if (`self.West`)
    ;[1 1 1] West
    (bind _returnvalue_5 (`AddComponent|NODE_AddInstancedStaticMeshComponent-8` :`RelativeTransform` (`KismetMathLibrary.MakeTransform` (`KismetMathLibrary.MakeVector` (`KismetMathLibrary.Conv_IntToDouble` (`local.LocalTotalLength`))) (struct :`Yaw` -270.0))))
    (for _index_9 (range (`self.Thickness`))
      (set `local.LocalThicknessIndex` _index_9)
      (for _index_10 (range (`self.Length`))
        (set `local.LocalLengthIndex` _index_10)
        (`InstancedStaticMeshComponent.AddInstance` _returnvalue_5 (`KismetMathLibrary.MakeTransform` (`KismetMathLibrary.MakeVector` 0.0 (`KismetMathLibrary.Conv_IntToDouble` (* (`local.LocalLengthIndex`) (`local.LocalTileSize`))) (`KismetMathLibrary.Conv_IntToDouble` (* (`local.LocalSideThickness`) (`local.LocalThicknessIndex`)))))))))
  (if (`self.Underside`)
    (bind _returnvalue_6 (`AddComponent|NODE_AddInstancedStaticMeshComponent-9` :`RelativeTransform` (`KismetMathLibrary.MakeTransform` (`KismetMathLibrary.MakeVector` (`KismetMathLibrary.Conv_IntToDouble` (`local.LocalTotalLength`)) 0.0 (`KismetMathLibrary.Conv_IntToDouble` (`local.LocalTotalThickness`))) (struct :`Pitch` 180.0))))
    (for _index_11 (range (`self.Width`))
      (set `local.LocalWidthIndex` _index_11)
      (for _index_12 (range (`self.Length`))
        (set `local.LocalLengthIndex` _index_12)
        (`InstancedStaticMeshComponent.AddInstance` _returnvalue_6 (`KismetMathLibrary.MakeTransform` (`KismetMathLibrary.MakeVector` (`KismetMathLibrary.Conv_IntToDouble` (* (`local.LocalLengthIndex`) _localtilesize)) (`KismetMathLibrary.Conv_IntToDouble` (* _localtilesize (`local.LocalWidthIndex`)))))))))
  ;[1 1 1] Cube transforms
  (`SceneComponent.K2_SetRelativeTransform` (`self.Cube1`) (`KismetMathLibrary.MakeTransform` (`KismetMathLibrary.MakeVector` (/ (`KismetMathLibrary.Conv_IntToDouble` (* (`self.Length`) (`local.LocalTileSize`))) 2.0) (/ (`KismetMathLibrary.Conv_IntToDouble` (* (`self.Width`) (`local.LocalTileSize`))) 2.0) (* (`local.LocalTotalThickness`) 0.5)) (struct) (`KismetMathLibrary.MakeVector` (- (`KismetMathLibrary.Conv_IntToDouble` (`self.Length`)) 0.01) (- (`KismetMathLibrary.Conv_IntToDouble` (`self.Width`)) 0.01) (- (* (`self.Thickness`) 0.05) 0.01))) false false)
  (if (`self.InsideBox`)
    (`SceneComponent.SetVisibility` _cube1 true false)
    (else
      (`SceneComponent.SetVisibility` _cube1 false false))))