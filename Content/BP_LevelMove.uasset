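; BP_LevelMove is an overlap-triggered actor that saves player progress, with no level change in its own graph.
; On any actor overlap it creates a fresh NewSaveGame and copies in gold from CardLordGameInstance and the item array of the first BP_MyCharacter found.
; It zeroes the saved reset position and writes the object to a fixed save slot, overwriting what was there.
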(event `self.ReceiveActorBeginOverlap`
  (params (OtherActor :type "Actor Object Reference"))
  (bind _returnvalue (`GameplayStatics.CreateSaveGameObject` "/Game/UI/SaveGame/NewSaveGame.NewSaveGame_C"))
  (bind _output_get (set `self.NewVar_0` _returnvalue))
  (bind _asnew_save_game (cast `/Game/UI/SaveGame/NewSaveGame` _output_get))
  (bind _ascard_lord_game_instance (cast `CardLordGameInstance` (`GameplayStatics.GetGameInstance`)))
  (bind _outactors (`GameplayStatics.GetAllActorsOfClass` "/Game/Character/Player/Blueprints/BP_MyCharacter.BP_MyCharacter_C"))
  (set `/Game/UI/SaveGame/NewSaveGame.Gold` (`CardLordGameInstance.GameGold` _ascard_lord_game_instance) _asnew_save_game)
  (set `/Game/UI/SaveGame/NewSaveGame.SaveInventory` (`/Game/Character/Player/Blueprints/BP_MyCharacter.ItemArray` (`|GetArrayItem` _outactors)) _asnew_save_game)
  (set `/Game/UI/SaveGame/NewSaveGame.PositionReset` (0.0 0.0 0.0) _asnew_save_game)
  (`GameplayStatics.SaveGameToSlot` _output_get "A"))

(fn `UserConstructionScript`)