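; Door teleport trigger that saves player state and opens the "Toilets" level when anything overlaps its box.
; With an existing slot "A" save, it updates the character's location as ToiletSpawn, plus camera state, and clears ReturnToHub.
; Otherwise it creates a NewSaveGame that also stores GameInstance gold and character inventory, with ToiletSpawn slightly offset from the trigger's location.
; Both branches save to the slot before loading the level.
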(event `self.Box.OnComponentBeginOverlap`
  (params (OverlappedComponent :type "PrimitiveComponent Object Reference") (OtherActor :type "Actor Object Reference") (OtherComp :type "PrimitiveComponent Object Reference") (OtherBodyIndex :type Integer) (bFromSweep :type Boolean) (SweepResult :type "HitResult Structure (by ref)"))
  (bind _returnvalue (`GameplayStatics.DoesSaveGameExist` "A"))
  (if _returnvalue
    (bind _returnvalue_2 (`GameplayStatics.LoadGameFromSlot` "A"))
    (bind _asnew_save_game (cast `/Game/UI/SaveGame/NewSaveGame` _returnvalue_2))
    (bind _outactors (`GameplayStatics.GetAllActorsOfClass` "/Game/Character/Player/Blueprints/BP_MyCharacter.BP_MyCharacter_C"))
    (bind _output (`|GetArrayItem` _outactors))
    (set `/Game/UI/SaveGame/NewSaveGame.ToiletSpawn` (`self.K2_GetActorLocation` _output) _asnew_save_game)
    (set `/Game/UI/SaveGame/NewSaveGame.SaveGameRotator` (`MyCharacter.SavedCameraFvector` _output) _asnew_save_game)
    (set `/Game/UI/SaveGame/NewSaveGame.CameraSwitcher` (`MyCharacter.CameraSwitch` _output) _asnew_save_game)
    (set `/Game/UI/SaveGame/NewSaveGame.ReturnToHub` false _asnew_save_game)
    (`GameplayStatics.SaveGameToSlot` _returnvalue_2 "A")
    (else
      (bind _returnvalue_3 (`GameplayStatics.CreateSaveGameObject` "/Game/UI/SaveGame/NewSaveGame.NewSaveGame_C"))
      (bind _output_get (set `self.NewVar_0` _returnvalue_3))
      (bind _asnew_save_game_2 (cast `/Game/UI/SaveGame/NewSaveGame` _output_get))
      (bind _ascard_lord_game_instance (cast `CardLordGameInstance` (`GameplayStatics.GetGameInstance`)))
      (bind _outactors_2 (`GameplayStatics.GetAllActorsOfClass` "/Game/Character/Player/Blueprints/BP_MyCharacter.BP_MyCharacter_C"))
      (set `/Game/UI/SaveGame/NewSaveGame.Gold` (`CardLordGameInstance.GameGold` _ascard_lord_game_instance) _asnew_save_game_2)
      (bind _output_2 (`|GetArrayItem` _outactors_2))
      (set `/Game/UI/SaveGame/NewSaveGame.SaveInventory` (`/Game/Character/Player/Blueprints/BP_MyCharacter.ItemArray` _output_2) _asnew_save_game_2)
      (set `/Game/UI/SaveGame/NewSaveGame.SaveGameRotator` (`MyCharacter.SavedCameraFvector` _output_2) _asnew_save_game_2)
      (bind _output_get_2 (set `/Game/UI/SaveGame/NewSaveGame.ToiletSpawn` (- (`self.K2_GetActorLocation`) (0.0 20.0 0.0)) _asnew_save_game_2))
      (`KismetSystemLibrary.PrintString` (`KismetStringLibrary.Conv_VectorToString` _output_get_2))
      (set `/Game/UI/SaveGame/NewSaveGame.CameraSwitcher` (`MyCharacter.CameraSwitch` _output_2) _asnew_save_game_2)
      (set `/Game/UI/SaveGame/NewSaveGame.ReturnToHub` false _asnew_save_game_2)
      (`GameplayStatics.SaveGameToSlot` _output_get "A")))
  (`GameplayStatics.OpenLevel` "Toilets"))

(fn `UserConstructionScript`)