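; Procedural cardboard floor tile Blueprint that sizes itself from Width and Length in the Construction Script; the event graph is empty.
; It scales the top FloorTile and places four side tiles around it, rotated in 90-degree steps.
; Dynamic instances of CardboardUniversal_MAT, one for the face and one per opposite side pair, scale tiling with dimensions to avoid stretching and enable the mask only on sides.
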(fn `UserConstructionScript`
  (locals (LocalTileSize :type Integer :default 100) (LocalSideThickness :type Integer :default 5) (LocalTotalWidth :type Integer) (LocalTotalLength :type Integer) (LocalTotalThickness :type Integer) (DynamicFaceMat :type "MaterialInstanceDynamic Object Reference") (DynamicSideMat_0 :type "MaterialInstanceDynamic Object Reference") (DynamicSideMat_1 :type "MaterialInstanceDynamic Object Reference") (CorrugationUTiling :type "Float (double-precision)" :default 15.0) (CorrugationVTiling :type "Float (double-precision)" :default 16.5) (FaceUTiling :type "Float (double-precision)" :default 1.0) (FaceVTiling :type "Float (double-precision)" :default 1.0))
  (bind _sidetile03 (`self.sideTile03`))
  (bind _sidetile04 (`self.sideTile04`))
  (bind _floortile (`self.floorTile`))
  (set `local.LocalTotalThickness` (* 0 (`local.LocalSideThickness`)))
  (set `local.LocalTotalWidth` (* (`self.Width`) (`local.LocalTileSize`)))
  (set `local.LocalTotalLength` (* (`self.Length`) (`local.LocalTileSize`)))
  (`|ExecutionSequence`
    (:`then_0`
      (`SceneComponent.SetRelativeScale3D` _floortile (`KismetMathLibrary.MakeVector` (`KismetMathLibrary.Conv_IntToDouble` (`self.Length`)) (`KismetMathLibrary.Conv_IntToDouble` (`self.Width`)) 1.0))
      (bind _returnvalue (`PrimitiveComponent.CreateDynamicMaterialInstance` _floortile 0 "/Game/Assets/Materials/TestMaterial/CardboardUniversal_MAT.CardboardUniversal_MAT" "None"))
      (bind _output_get (set `local.DynamicFaceMat` _returnvalue))
      (`|ExecutionSequence`
        (:`then_0`
          (`MaterialInstanceDynamic.SetScalarParameterValue` _output_get "CorrugationUTiling" (* (`local.CorrugationUTiling`) 1.0)))
        (:`then_1`
          (`MaterialInstanceDynamic.SetScalarParameterValue` _output_get "CorrugationVTiling" (* (`local.CorrugationVTiling`) 1.0)))
        (:`then_2`
          (`MaterialInstanceDynamic.SetScalarParameterValue` _output_get "FaceUTiling" (* (`local.FaceUTiling`) (`KismetMathLibrary.Conv_IntToDouble` (`self.Length`)))))
        (:`then_3`
          (`MaterialInstanceDynamic.SetScalarParameterValue` _output_get "FaceVTiling" (* (`local.FaceVTiling`) (`KismetMathLibrary.Conv_IntToDouble` (`self.Width`)))))
        (:`then_4`
          (`MaterialInstanceDynamic.SetScalarParameterValue` _output_get "U_Offset" (* 0.0 1.0)))
        (:`then_5`
          (`MaterialInstanceDynamic.SetScalarParameterValue` _output_get "V_Offset" (* 0.0 1.0)))
        (:`then_6`
          (`MaterialInstanceDynamic.SetScalarParameterValue` _output_get "UseMask" 0.0))))
    (:`then_1`
      ;[1 1 1] 1
      (`SceneComponent.K2_SetRelativeTransform` (`self.sideTile01`) (`KismetMathLibrary.MakeTransform` (0.0 0.0 0.0) (struct) (`KismetMathLibrary.MakeVector` (`KismetMathLibrary.Conv_IntToDouble` (`self.Length`)) (`KismetMathLibrary.Conv_IntToDouble` (`self.Width`)) 2.0)) false false)
      ;[1 1 1] 3
      (`SceneComponent.K2_SetRelativeTransform` _sidetile03 (`KismetMathLibrary.MakeTransform` (`KismetMathLibrary.MakeVector` (`KismetMathLibrary.Conv_IntToDouble` (`local.LocalTotalLength`)) (`KismetMathLibrary.Conv_IntToDouble` (`local.LocalTotalWidth`))) (struct :`Yaw` 180.0) (`KismetMathLibrary.MakeVector` (`KismetMathLibrary.Conv_IntToDouble` (`self.Length`)) (`KismetMathLibrary.Conv_IntToDouble` (`self.Width`)) 2.0)) false false)
      (bind _returnvalue_2 (`PrimitiveComponent.CreateDynamicMaterialInstance` _sidetile03 0 "/Game/Assets/Materials/TestMaterial/CardboardUniversal_MAT.CardboardUniversal_MAT" "None"))
      (bind _output_get_2 (set `local.DynamicSideMat_0` _returnvalue_2))
      (`PrimitiveComponent.SetMaterial` (`self.sideTile01`) 0 _output_get_2)
      (`PrimitiveComponent.SetMaterial` (`self.sideTile03`) 0 _output_get_2)
      (`|ExecutionSequence`
        (:`then_0`
          (`MaterialInstanceDynamic.SetScalarParameterValue` _output_get_2 "CorrugationUTiling" (* (+ (`self.U_Offset`) 1.0) (* (`local.CorrugationUTiling`) (`KismetMathLibrary.Conv_IntToDouble` (`self.Width`))))))
        (:`then_1`
          (`MaterialInstanceDynamic.SetScalarParameterValue` _output_get_2 "CorrugationVTiling" (* (`local.CorrugationVTiling`) (`KismetMathLibrary.Conv_IntToDouble` 2))))
        (:`then_2`
          (`MaterialInstanceDynamic.SetScalarParameterValue` _output_get_2 "U_Offset" 0.0))
        (:`then_3`
          (`MaterialInstanceDynamic.SetScalarParameterValue` _output_get_2 "V_Offset" (`self.V_Offset`)))
        (:`then_4`
          (`MaterialInstanceDynamic.SetScalarParameterValue` _output_get_2 "UseMask" 1.0))))
    (:`then_2`
      ;[1 1 1] 2
      (`SceneComponent.K2_SetRelativeTransform` (`self.sideTile02`) (`KismetMathLibrary.MakeTransform` (`KismetMathLibrary.MakeVector` 0.0 (`KismetMathLibrary.Conv_IntToDouble` (`local.LocalTotalWidth`))) (struct :`Yaw` 270.0) (`KismetMathLibrary.MakeVector` (`KismetMathLibrary.Conv_IntToDouble` (`self.Width`)) (`KismetMathLibrary.Conv_IntToDouble` (`self.Length`)) 2.0)) false false)
      ;[1 1 1] 4
      (`SceneComponent.K2_SetRelativeTransform` _sidetile04 (`KismetMathLibrary.MakeTransform` (`KismetMathLibrary.MakeVector` (`KismetMathLibrary.Conv_IntToDouble` (`local.LocalTotalLength`))) (struct :`Yaw` 90.0) (`KismetMathLibrary.MakeVector` (`KismetMathLibrary.Conv_IntToDouble` (`self.Width`)) (`KismetMathLibrary.Conv_IntToDouble` (`self.Length`)) 2.0)) false false)
      (bind _returnvalue_3 (`PrimitiveComponent.CreateDynamicMaterialInstance` _sidetile04 0 "/Game/Assets/Materials/TestMaterial/CardboardUniversal_MAT.CardboardUniversal_MAT" "None"))
      (bind _output_get_3 (set `local.DynamicSideMat_1` _returnvalue_3))
      (`PrimitiveComponent.SetMaterial` (`self.sideTile04`) 0 _output_get_3)
      (`PrimitiveComponent.SetMaterial` (`self.sideTile02`) 0 _output_get_3)
      (`|ExecutionSequence`
        (:`then_0`
          (`MaterialInstanceDynamic.SetScalarParameterValue` _output_get_3 "CorrugationUTiling" (* (+ (`self.U_Offset`) 1.0) (* (`local.CorrugationUTiling`) (`KismetMathLibrary.Conv_IntToDouble` (`self.Length`))))))
        (:`then_1`
          (`MaterialInstanceDynamic.SetScalarParameterValue` _output_get_3 "CorrugationVTiling" (* (`local.CorrugationVTiling`) (`KismetMathLibrary.Conv_IntToDouble` 2))))
        (:`then_2`
          (`MaterialInstanceDynamic.SetScalarParameterValue` _output_get_3 "U_Offset" 0.0))
        (:`then_3`
          (`MaterialInstanceDynamic.SetScalarParameterValue` _output_get_3 "V_Offset" (`self.V_Offset`)))
        (:`then_4`
          (`MaterialInstanceDynamic.SetScalarParameterValue` _output_get_3 "UseMask" 1.0))))))