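; Point light actor with configurable color and intensity that can flicker on and off during play.
; The Construction Script applies the intensity, while the color is only applied at BeginPlay.
; When Flickering is enabled, BeginPlay starts an endless Delay loop that toggles the light's visibility at random intervals between the minimum and maximum flicker speeds, which act as seconds between toggles.
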(event `self.ReceiveBeginPlay`
  (`LightComponent.SetLightColor` (`self.PointLight`) (`self.LightColor`) true)
  (if (`self.Flickering`)
    (`SceneComponent.SetVisibility` (`self.PointLight`) (`self.LightOn`) false :!label _label)
    (`KismetSystemLibrary.Delay` (`KismetMathLibrary.RandomFloatInRange` (`self.Flicker speed Min`) (`self.Flicker speed Max`)))
    (set `self.LightOn` (not (`self.LightOn`)))
    (goto _label)))

(fn `UserConstructionScript`
  (`LightComponent.SetIntensity` (`self.PointLight`) (`self.Light intensity`)))