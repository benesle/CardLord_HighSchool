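; BP_MyNerd is an enemy actor that saves the game when a MyCharacter overlaps it.
; The overlap sets the character's PositionReset to the player controller's location with a small Y offset.
; It then writes gold from CardLordGameInstance, plus inventory and PositionReset from the first BP_MyCharacter, into a new NewSaveGame in slot "A".
; A capsule overlap caches the player reference, which is never cleared or used here.
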(event `self.ReceiveActorBeginOverlap`
  (params (OtherActor :type "Actor Object Reference"))
  (bind _asmy_character (cast `MyCharacter` OtherActor))
  (set `MyCharacter.PositionReset` (- (`self.K2_GetActorLocation` (`GameplayStatics.GetPlayerController` 0)) (0.0 10.0 0.0)) _asmy_character)
  (bind _returnvalue (`GameplayStatics.CreateSaveGameObject` "/Game/UI/SaveGame/NewSaveGame.NewSaveGame_C"))
  (bind _asnew_save_game (cast `/Game/UI/SaveGame/NewSaveGame` _returnvalue))
  (bind _output_get (set `self.SavingEnemy1` _asnew_save_game))
  (bind _ascard_lord_game_instance (cast `CardLordGameInstance` (`GameplayStatics.GetGameInstance`)))
  (bind _outactors (`GameplayStatics.GetAllActorsOfClass` "/Game/Character/Player/Blueprints/BP_MyCharacter.BP_MyCharacter_C"))
  (set `/Game/UI/SaveGame/NewSaveGame.Gold` (`CardLordGameInstance.GameGold` _ascard_lord_game_instance) _asnew_save_game)
  (bind _output (`|GetArrayItem` _outactors))
  (set `/Game/UI/SaveGame/NewSaveGame.SaveInventory` (`/Game/Character/Player/Blueprints/BP_MyCharacter.ItemArray` _output) _asnew_save_game)
  (set `/Game/UI/SaveGame/NewSaveGame.PositionReset` (`MyCharacter.PositionReset` _output) _asnew_save_game)
  (`GameplayStatics.SaveGameToSlot` _output_get "A"))

(event `self.Capsule_0.OnComponentBeginOverlap`
  (params (OverlappedComponent :type "PrimitiveComponent Object Reference") (OtherActor :type "Actor Object Reference") (OtherComp :type "PrimitiveComponent Object Reference") (OtherBodyIndex :type Integer) (bFromSweep :type Boolean) (SweepResult :type "HitResult Structure (by ref)"))
  (bind _asbp_my_character (cast `/Game/Character/Player/Blueprints/BP_MyCharacter` OtherActor))
  (set `self.PlayerCharacter` _asbp_my_character))

(event `self.Capsule_0.OnComponentEndOverlap`
  (params (OverlappedComponent :type "PrimitiveComponent Object Reference") (OtherActor :type "Actor Object Reference") (OtherComp :type "PrimitiveComponent Object Reference") (OtherBodyIndex :type Integer))
  (cast `/Game/Character/Player/Blueprints/BP_MyCharacter` OtherActor))

(fn `UserConstructionScript`)