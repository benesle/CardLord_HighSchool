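; Door teleport trigger, apparently leaving the second toilet, that saves progress and sends the player to Hallway_Floor1.
; Any Box overlap loads save slot A, then copies in gold from the game instance plus inventory and camera state from the first BP_MyCharacter.
; It flags ReturnToHub, saves the slot and shows a loading screen before opening the level.
; The overlapping actor is not checked, and ToiletSpawn is only assigned to itself.
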(event `self.Box.OnComponentBeginOverlap`
  (params (OverlappedComponent :type "PrimitiveComponent Object Reference") (OtherActor :type "Actor Object Reference") (OtherComp :type "PrimitiveComponent Object Reference") (OtherBodyIndex :type Integer) (bFromSweep :type Boolean) (SweepResult :type "HitResult Structure (by ref)"))
  (bind _returnvalue (`GameplayStatics.LoadGameFromSlot` "A"))
  (bind _asnew_save_game (cast `/Game/UI/SaveGame/NewSaveGame` _returnvalue))
  (bind _ascard_lord_game_instance (cast `CardLordGameInstance` (`GameplayStatics.GetGameInstance`)))
  (bind _outactors (`GameplayStatics.GetAllActorsOfClass` "/Game/Character/Player/Blueprints/BP_MyCharacter.BP_MyCharacter_C"))
  (set `/Game/UI/SaveGame/NewSaveGame.Gold` (`CardLordGameInstance.GameGold` _ascard_lord_game_instance) _asnew_save_game)
  (bind _output (`|GetArrayItem` _outactors))
  (set `/Game/UI/SaveGame/NewSaveGame.SaveInventory` (`/Game/Character/Player/Blueprints/BP_MyCharacter.ItemArray` _output) _asnew_save_game)
  (set `/Game/UI/SaveGame/NewSaveGame.ToiletSpawn` (`/Game/UI/SaveGame/NewSaveGame.ToiletSpawn` _asnew_save_game) _asnew_save_game)
  (set `/Game/UI/SaveGame/NewSaveGame.SaveGameRotator` (`MyCharacter.SavedCameraFvector` _output) _asnew_save_game)
  (set `/Game/UI/SaveGame/NewSaveGame.CameraSwitcher` (`MyCharacter.CameraSwitch` _output) _asnew_save_game)
  (set `/Game/UI/SaveGame/NewSaveGame.ReturnToHub` true _asnew_save_game)
  (`KismetSystemLibrary.PrintString` "Hello")
  (`GameplayStatics.SaveGameToSlot` _returnvalue "A")
  (bind _returnvalue_2 (`|CreateWidget` "/Game/Assets/Blueprints/DoorTeleports/Loading_Screen.Loading_Screen_C"))
  (`UserWidget.AddToViewport` _returnvalue_2 0)
  (`GameplayStatics.OpenLevel` "Hallway_Floor1" false))

(fn `UserConstructionScript`)