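; WallSection_BP is a procedural wall section, built entirely in the construction script from tiled instanced meshes sized by Width, Height and Thickness.
; Front and mirrored back faces share one instanced component, with the back offset by Thickness times SideThickness.
; NoEndPieces, ASide and BSide control the end caps, while top pieces are always added.
; Each end and top piece gets its own instanced component, so those pieces are not batched.
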(fn `UserConstructionScript`
  (bind _tilesize (`self.TileSize`))
  (bind _widthloopindex (`self.WidthLoopIndex`))
  (bind _returnvalue (`AddComponent|NODE_AddInstancedStaticMeshComponent-2`))
  (for _index (range (`self.Width`))
    (bind _output_get (set `self.WidthLoopIndex` _index))
    (for _index_2 (range (`self.Height`))
      (set `self.HeightLoopIndex` _index_2)
      (`InstancedStaticMeshComponent.AddInstance` _returnvalue (`KismetMathLibrary.MakeTransform` (`KismetMathLibrary.MakeVector` 0.0 (`KismetMathLibrary.Conv_IntToDouble` (* _output_get (`self.TileSize`))) (`KismetMathLibrary.Conv_IntToDouble` (* _index_2 (`self.TileSize`)))) (`KismetMathLibrary.MakeRotator` 0.0 (`KismetMathLibrary.Conv_IntToDouble` (`self.InitialRotation`)))))
      (`InstancedStaticMeshComponent.AddInstance` _returnvalue (`KismetMathLibrary.MakeTransform` (`KismetMathLibrary.MakeVector` (`KismetMathLibrary.Conv_IntToDouble` (* (`self.Thickness`) (`self.sideThickness`))) (`KismetMathLibrary.Conv_IntToDouble` (* (+ (`self.WidthLoopIndex`) 1) (`self.TileSize`))) (`KismetMathLibrary.Conv_IntToDouble` (* (`self.HeightLoopIndex`) (`self.TileSize`)))) (`KismetMathLibrary.MakeRotator` 0.0 90.0 180.0)))
      (if (not (`self.NoEndPieces`))
        (if (== _widthloopindex 0)
          (for _index_3 (range (`self.Thickness`))
            (if (`self.A_Side`)
              (bind _returnvalue_2 (`AddComponent|NODE_AddInstancedStaticMeshComponent-3`))
              (`InstancedStaticMeshComponent.AddInstance` _returnvalue_2 (`KismetMathLibrary.MakeTransform` (`KismetMathLibrary.MakeVector` (`KismetMathLibrary.Conv_IntToDouble` (* (+ _index_3 1) (`self.sideThickness`))) 0.0 (`KismetMathLibrary.Conv_IntToDouble` (* (`self.HeightLoopIndex`) (`self.TileSize`)))) (`KismetMathLibrary.MakeRotator` -90.0 0.0 90.0))))))
        (if (`self.B_Side`)
          (if (== _widthloopindex (- (`self.Width`) 1))
            (for _index_4 (range (`self.Thickness`))
              (bind _returnvalue_3 (`AddComponent|NODE_AddInstancedStaticMeshComponent-4`))
              (`InstancedStaticMeshComponent.AddInstance` _returnvalue_3 (`KismetMathLibrary.MakeTransform` (`KismetMathLibrary.MakeVector` (`KismetMathLibrary.Conv_IntToDouble` (* _index_4 (`self.sideThickness`))) (`KismetMathLibrary.Conv_IntToDouble` (* (`self.TileSize`) (`self.Width`))) (`KismetMathLibrary.Conv_IntToDouble` (* (`self.HeightLoopIndex`) (`self.TileSize`)))) (`KismetMathLibrary.MakeRotator` -90.0 0.0 -90.0)))))))))
  (for _index_5 (range (`self.Thickness`))
    (for _index_6 (range (`self.Width`))
      (bind _returnvalue_4 (`AddComponent|NODE_AddInstancedStaticMeshComponent-5`))
      (`InstancedStaticMeshComponent.AddInstance` _returnvalue_4 (`KismetMathLibrary.MakeTransform` (`KismetMathLibrary.MakeVector` (`KismetMathLibrary.Conv_IntToDouble` (* _index_5 (`self.sideThickness`))) (`KismetMathLibrary.Conv_IntToDouble` (- (* (`self.Width`) (`self.TileSize`)) (* _index_6 _tilesize))) (`KismetMathLibrary.Conv_IntToDouble` (* _tilesize (`self.Height`)))) (`KismetMathLibrary.MakeRotator` 180.0 -90.0))))))