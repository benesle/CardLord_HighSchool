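; Newtiles is a resizable tile piece actor that sets itself up in the construction script, with no active event graph logic.
; Length and Width scale the tile mesh in X and Y, leaving Z at one.
; A dynamic instance of the tile material gets face tiling multiplied by each matching dimension and corrugation U tiling by their average, so textures follow the size.
; Corrugation V tiling and UV offsets pass through unscaled.
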(fn `UserConstructionScript`
  (locals (ParamNamesVar :type Name) (CorrugationUTiling :type "Float (double-precision)" :default 60.0) (CorrugationVTiling :type "Float (double-precision)" :default 80.0) (FaceUTiling :type "Float (double-precision)" :default 1.0) (FaceVTiling :type "Float (double-precision)" :default 1.0) (U_Offset :type "Float (double-precision)" :default 0.0) (V_Offset :type "Float (double-precision)") (LocalDynamicMat :type "MaterialInstanceDynamic Object Reference"))
  (bind _newtilepiece_fbx (`self.NewTilePiece_FBX`))
  (`SceneComponent.SetRelativeScale3D` _newtilepiece_fbx (`KismetMathLibrary.MakeVector` (`self.Length`) (`self.Width`) 1.0))
  (bind _returnvalue (`PrimitiveComponent.CreateDynamicMaterialInstance` _newtilepiece_fbx 0 "/Game/Assets/Materials/TestMaterial/NewTile_MAT_Inst.NewTile_MAT_Inst" "None"))
  (bind _output_get (set `local.LocalDynamicMat` _returnvalue))
  (`|ExecutionSequence`
    (:`then_0`
      (`MaterialInstanceDynamic.SetScalarParameterValue` _output_get "CorrugationUTiling" (* (`local.CorrugationUTiling`) (/ (+ (`self.Length`) (`self.Width`)) 2.0))))
    (:`then_1`
      (`MaterialInstanceDynamic.SetScalarParameterValue` _output_get "CorrugationVTiling" (* (`local.CorrugationVTiling`) 1.0)))
    (:`then_2`
      (`MaterialInstanceDynamic.SetScalarParameterValue` _output_get "FaceUTiling" (* (`local.FaceUTiling`) (`self.Length`))))
    (:`then_3`
      (`MaterialInstanceDynamic.SetScalarParameterValue` _output_get "FaceVTiling" (* (`local.FaceVTiling`) (`self.Width`))))
    (:`then_4`
      (`MaterialInstanceDynamic.SetScalarParameterValue` _output_get "U_Offset" (* (`local.U_Offset`) 1.0)))
    (:`then_5`
      (`MaterialInstanceDynamic.SetScalarParameterValue` _output_get "V_Offset" (* (`local.V_Offset`) 1.0)))))