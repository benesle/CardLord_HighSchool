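; Loot locker prop with six doors, one of which is picked at random to swing open when the player loots it.
; BeginPlay rolls the door and rotates it to an initial yaw; player overlap with the box sets Looting and, after a short delay, eases that door to the open rotation.
; Per-door macros wrap MoveComponentTo; leaving the box only clears Looting.
; The construction script tints door A1 red via a dynamic material.
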(event `self.ReceiveBeginPlay`
  (bind _lootspeed (`self.LootSpeed`))
  (bind _randomdoor (`self.RandomDoor`))
  (bind _initrotation (`self.InitRotation`))
  (set `self.RandomDoor` (`KismetMathLibrary.RandomInteger` 6))
  (if (== _randomdoor 0)
    (`self.A1_Macro` _lootspeed _initrotation)
    (elif (== _randomdoor 1)
      (`self.A2_Macro` _lootspeed _initrotation)
      (elif (== _randomdoor 2)
        (`self.A3_Macro` _lootspeed _initrotation)
        (elif (== _randomdoor 3)
          (`self.B1_Macro` _lootspeed _initrotation)
          (elif (== _randomdoor 4)
            (`self.B2_Macro` _lootspeed _initrotation)
            (elif (== _randomdoor 5)
              (`self.B3_Macro` _lootspeed _initrotation))))))))

(event `self.Box.OnComponentBeginOverlap`
  (params (OverlappedComponent :type "PrimitiveComponent Object Reference") (OtherActor :type "Actor Object Reference") (OtherComp :type "PrimitiveComponent Object Reference") (OtherBodyIndex :type Integer) (bFromSweep :type Boolean) (SweepResult :type "HitResult Structure (by ref)"))
  (bind _lootspeed (`self.LootSpeed`))
  (bind _randomdoor (`self.RandomDoor`))
  (bind _rotationamnt (`self.RotationAmnt`))
  (cast `MyCharacter` OtherActor)
  (cast `CardLordGameInstance` (`GameplayStatics.GetGameInstance`))
  (set `self.Looting` true)
  (`KismetSystemLibrary.Delay` 0.4)
  (if (== _randomdoor 0)
    (`self.A1_Macro` _lootspeed _rotationamnt)
    (elif (== _randomdoor 1)
      (`self.A2_Macro` _lootspeed _rotationamnt)
      (elif (== _randomdoor 2)
        (`self.A3_Macro` _lootspeed _rotationamnt)
        (elif (== _randomdoor 3)
          (`self.B1_Macro` _lootspeed _rotationamnt)
          (elif (== _randomdoor 4)
            (`self.B2_Macro` _lootspeed _rotationamnt)
            (elif (== _randomdoor 5)
              (`self.B3_Macro` _lootspeed _rotationamnt))))))))

(event `self.Box.OnComponentEndOverlap`
  (params (OverlappedComponent :type "PrimitiveComponent Object Reference") (OtherActor :type "Actor Object Reference") (OtherComp :type "PrimitiveComponent Object Reference") (OtherBodyIndex :type Integer))
  (cast `MyCharacter` OtherActor)
  (cast `CardLordGameInstance` (`GameplayStatics.GetGameInstance`))
  (set `self.Looting` false))

(fn `UserConstructionScript`
  (bind _returnvalue (`KismetMaterialLibrary.CreateDynamicMaterialInstance` "/Game/Assets/Materials/TestMaterial/LockerDoor_MAT_Inst.LockerDoor_MAT_Inst"))
  (`MaterialInstanceDynamic.SetVectorParameterValue` _returnvalue "Color" (`KismetMathLibrary.MakeColor` 0.9 0.1 0.1))
  (`PrimitiveComponent.SetMaterial` (`self.Lockers_DoorA1`) 0 _returnvalue))