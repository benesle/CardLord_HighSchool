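; Actor component that moves the player between levels, carrying state across through the NewSaveGame in slot "A".
; TeleportTo updates the save with player location and camera, or creates one with gold, inventory and an owner-offset spawn, then opens the level.
; TeleportBack saves gold, inventory and camera, keeps the stored spawn, flags ReturnToHub and shows a loading screen before opening the level.
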(fn `TeleportBack`
  (params (LevemName :type Name))
  (bind _returnvalue (`GameplayStatics.LoadGameFromSlot` "A"))
  (bind _asnew_save_game (cast `/Game/UI/SaveGame/NewSaveGame` _returnvalue))
  (bind _ascard_lord_game_instance (cast `CardLordGameInstance` (`GameplayStatics.GetGameInstance`)))
  (bind _outactors (`GameplayStatics.GetAllActorsOfClass` "/Game/Character/Player/Blueprints/BP_MyCharacter.BP_MyCharacter_C"))
  (set `/Game/UI/SaveGame/NewSaveGame.Gold` (`CardLordGameInstance.GameGold` _ascard_lord_game_instance) _asnew_save_game)
  (bind _output (`|GetArrayItem` _outactors))
  (set `/Game/UI/SaveGame/NewSaveGame.SaveInventory` (`/Game/Character/Player/Blueprints/BP_MyCharacter.ItemArray` _output) _asnew_save_game)
  (set `/Game/UI/SaveGame/NewSaveGame.ToiletSpawn` (`/Game/UI/SaveGame/NewSaveGame.ToiletSpawn` _asnew_save_game) _asnew_save_game)
  (set `/Game/UI/SaveGame/NewSaveGame.SaveGameRotator` (`MyCharacter.SavedCameraFvector` _output) _asnew_save_game)
  (set `/Game/UI/SaveGame/NewSaveGame.CameraSwitcher` (`MyCharacter.CameraSwitch` _output) _asnew_save_game)
  (set `/Game/UI/SaveGame/NewSaveGame.ReturnToHub` true _asnew_save_game)
  (`KismetSystemLibrary.PrintString` "Hello")
  (`GameplayStatics.SaveGameToSlot` _returnvalue "A")
  (bind _returnvalue_2 (`|CreateWidget` "/Game/Assets/Blueprints/DoorTeleports/Loading_Screen.Loading_Screen_C"))
  (`UserWidget.AddToViewport` _returnvalue_2 0)
  (`GameplayStatics.OpenLevel` LevemName false))

(fn `TeleportTo`
  (params (LevelName :type Name) (`Teleport Offset` :type "Vector Structure"))
  (bind _returnvalue (`GameplayStatics.DoesSaveGameExist` "A"))
  (if _returnvalue
    (bind _returnvalue_2 (`GameplayStatics.LoadGameFromSlot` "A"))
    (bind _asnew_save_game (cast `/Game/UI/SaveGame/NewSaveGame` _returnvalue_2))
    (bind _outactors (`GameplayStatics.GetAllActorsOfClass` "/Game/Character/Player/Blueprints/BP_MyCharacter.BP_MyCharacter_C"))
    (bind _output (`|GetArrayItem` _outactors))
    (set `/Game/UI/SaveGame/NewSaveGame.ToiletSpawn` (`Actor.K2_GetActorLocation` _output) _asnew_save_game)
    (set `/Game/UI/SaveGame/NewSaveGame.SaveGameRotator` (`MyCharacter.SavedCameraFvector` _output) _asnew_save_game)
    (set `/Game/UI/SaveGame/NewSaveGame.CameraSwitcher` (`MyCharacter.CameraSwitch` _output) _asnew_save_game)
    (set `/Game/UI/SaveGame/NewSaveGame.ReturnToHub` false _asnew_save_game)
    (`GameplayStatics.SaveGameToSlot` _returnvalue_2 "A")
    (else
      (bind _returnvalue_3 (`GameplayStatics.CreateSaveGameObject` "/Game/UI/SaveGame/NewSaveGame.NewSaveGame_C"))
      (bind _output_get (set `self.NewVar_0` _returnvalue_3))
      (bind _asnew_save_game_2 (cast `/Game/UI/SaveGame/NewSaveGame` _output_get))
      (bind _ascard_lord_game_instance (cast `CardLordGameInstance` (`GameplayStatics.GetGameInstance`)))
      (bind _outactors_2 (`GameplayStatics.GetAllActorsOfClass` "/Game/Character/Player/Blueprints/BP_MyCharacter.BP_MyCharacter_C"))
      (set `/Game/UI/SaveGame/NewSaveGame.Gold` (`CardLordGameInstance.GameGold` _ascard_lord_game_instance) _asnew_save_game_2)
      (bind _output_2 (`|GetArrayItem` _outactors_2))
      (set `/Game/UI/SaveGame/NewSaveGame.SaveInventory` (`/Game/Character/Player/Blueprints/BP_MyCharacter.ItemArray` _output_2) _asnew_save_game_2)
      (set `/Game/UI/SaveGame/NewSaveGame.SaveGameRotator` (`MyCharacter.SavedCameraFvector` _output_2) _asnew_save_game_2)
      (bind _output_get_2 (set `/Game/UI/SaveGame/NewSaveGame.ToiletSpawn` (+ (`Actor.K2_GetActorLocation` (`self.GetOwner`)) `Teleport Offset`) _asnew_save_game_2))
      (`KismetSystemLibrary.PrintString` (`KismetStringLibrary.Conv_VectorToString` _output_get_2))
      (set `/Game/UI/SaveGame/NewSaveGame.CameraSwitcher` (`MyCharacter.CameraSwitch` _output_2) _asnew_save_game_2)
      (set `/Game/UI/SaveGame/NewSaveGame.ReturnToHub` false _asnew_save_game_2)
      (`GameplayStatics.SaveGameToSlot` _output_get "A")))
  (`GameplayStatics.OpenLevel` LevelName))