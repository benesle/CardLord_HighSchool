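; SideTiles_BP is a construction-time Blueprint that builds a grid of side tiles, forming a vertical strip.
; Its construction script adds one Instanced Static Mesh component and fills it through nested loops over Length and Thickness.
; Instances step along Y by TileSize and stack downward in Z by TileHeight.
; The event graph holds only disabled default events, so it has no runtime logic.
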(fn `UserConstructionScript`
  (bind _returnvalue (`AddComponent|NODE_AddInstancedStaticMeshComponent-2`))
  (for _index (range (`self.Length`))
    (for _index_2 (range (`self.Thickness`))
      (`InstancedStaticMeshComponent.AddInstance` _returnvalue (`KismetMathLibrary.MakeTransform` (`KismetMathLibrary.MakeVector` 0.0 (`KismetMathLibrary.Conv_IntToDouble` (* _index (`self.TileSize`))) (`KismetMathLibrary.Conv_IntToDouble` (* _index_2 (* (`self.TileHeight`) -1)))))))))