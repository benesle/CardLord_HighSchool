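; Bookshelf Blueprint that procedurally lays out a line of alternating mesh units in its Construction Script, with no active gameplay logic.
; A loop over Rows uses FlipFlops to alternate two instanced mesh types, stepping along X by gap variables at HeightOffset.
; ChangeDirection reverses the stepping, and SwitchOrder swaps which type leads and resets the start offset.
; One type shares a single component, while the other adds a new component per instance.
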(fn `UserConstructionScript`
  (locals (RowIndex :type Integer) (UnitGap1 :type "Float (double-precision)" :default 100.0) (HeightOffset :type "Float (double-precision)" :default -16.757446) (`Cumulative transform` :type "Float (double-precision)") (UnitGap2 :type "Float (double-precision)" :default 97.300003) (Direction :type "Float (double-precision)" :default 1.0) (UnitGap3 :type "Float (double-precision)" :default 97.300003))
  (bind _cumulative_transform (`local.Cumulative transform`))
  (bind _heightoffset (`local.HeightOffset`))
  (bind _cumulative_transform_2 (`local.Cumulative transform`))
  (bind _heightoffset_2 (`local.HeightOffset`))
  (if (`self.ChangeDirection`)
    (set `local.Direction` -1.0))
  (bind _returnvalue (`AddComponent|NODE_AddInstancedStaticMeshComponent-2`))
  (for _index (range (`self.Rows`))
    (if (`self.ChangeDirection`)
      ;[1 1 1] Reversed
      (if (and (`self.SwitchOrder`) (== _index 0))
        (set `local.Cumulative transform` -1.4))
      (if (`self.SwitchOrder`)
        (`/Engine/EditorBlueprintResources/StandardMacros.FlipFlop`
          (:`A`
            (bind _returnvalue_2 (`AddComponent|NODE_AddInstancedStaticMeshComponent-5` :!label _label))
            (`InstancedStaticMeshComponent.AddInstance` _returnvalue_2 (`KismetMathLibrary.MakeTransform` (`KismetMathLibrary.MakeVector` _cumulative_transform 0.0 _heightoffset_2)))
            (set `local.Cumulative transform` (- (`local.Cumulative transform`) (`local.UnitGap3`))))
          (:`B`
            (`InstancedStaticMeshComponent.AddInstance` _returnvalue (`KismetMathLibrary.MakeTransform` (`KismetMathLibrary.MakeVector` _cumulative_transform 0.0 _heightoffset_2)) :!label _label_2)
            (set `local.Cumulative transform` (- (`local.Cumulative transform`) (`local.UnitGap1`)))))
        (else
          (`/Engine/EditorBlueprintResources/StandardMacros.FlipFlop`
            (:`A`
              (goto _label_2))
            (:`B`
              (goto _label)))))
      (else
        ;[1 1 1] Not reversed
        (if (and (`self.SwitchOrder`) (== _index 0))
          (set `local.Cumulative transform` -1.4))
        (if (`self.SwitchOrder`)
          (`/Engine/EditorBlueprintResources/StandardMacros.FlipFlop`
            (:`A`
              (bind _returnvalue_3 (`AddComponent|NODE_AddInstancedStaticMeshComponent-4` :!label _label_3))
              (`InstancedStaticMeshComponent.AddInstance` _returnvalue_3 (`KismetMathLibrary.MakeTransform` (`KismetMathLibrary.MakeVector` _cumulative_transform_2 0.0 _heightoffset)))
              (set `local.Cumulative transform` (+ (`local.UnitGap1`) (`local.Cumulative transform`))))
            (:`B`
              (`InstancedStaticMeshComponent.AddInstance` _returnvalue (`KismetMathLibrary.MakeTransform` (`KismetMathLibrary.MakeVector` _cumulative_transform_2 0.0 _heightoffset)) :!label _label_4)
              (set `local.Cumulative transform` (+ (`local.UnitGap2`) (`local.Cumulative transform`)))))
          (else
            (`/Engine/EditorBlueprintResources/StandardMacros.FlipFlop`
              (:`A`
                (goto _label_4))
              (:`B`
                (goto _label_3)))))))))