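; Interactive toilet prop with a tintable material and a lid that reflects whether it holds loot.
; Without loot the lid is set open at BeginPlay; with loot, pressing E smoothly rotates it open.
; A box overlap toggles the actor's player input, without filtering the overlapping actor.
; The construction script tints a dynamic material, sharing it with the lid only when the side-color override is on.
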(event `self.ReceiveBeginPlay`
  ;[1 1 1] Loot state
  (if (not (`self.HasLoot`))
    (`SceneComponent.K2_SetRelativeRotation` (`self.Toilet_Lid_FBX`) (struct :`Pitch` 95.0) false false)))

(event `self.Box.OnComponentBeginOverlap`
  (params (OverlappedComponent :type "PrimitiveComponent Object Reference") (OtherActor :type "Actor Object Reference") (OtherComp :type "PrimitiveComponent Object Reference") (OtherBodyIndex :type Integer) (bFromSweep :type Boolean) (SweepResult :type "HitResult Structure (by ref)"))
  ;[1 1 1] Enable/Disable Input
  (`self.EnableInput` (`GameplayStatics.GetPlayerController` 0)))

(event `self.Box.OnComponentEndOverlap`
  (params (OverlappedComponent :type "PrimitiveComponent Object Reference") (OtherActor :type "Actor Object Reference") (OtherComp :type "PrimitiveComponent Object Reference") (OtherBodyIndex :type Integer))
  ;[1 1 1] Enable/Disable Input
  (`self.DisableInput` (`GameplayStatics.GetPlayerController` 0)))

(event `Key|E`
  (params (Key :type "Key Structure"))
  ;[1 1 1] Button press
  (:`Pressed`
    (if (`self.HasLoot`)
      (`KismetSystemLibrary.MoveComponentTo` (`self.Toilet_Lid_FBX`) (0.0 0.0 0.0) (struct :`Pitch` 95.0) true true 1.0 true))))

(fn `UserConstructionScript`
  (locals (ToiletMaterial :type "MaterialInstanceDynamic Object Reference"))
  (bind _returnvalue (`PrimitiveComponent.CreateDynamicMaterialInstance` (`self.Toilet_FBX`) 0 "/Game/Assets/Materials/Toilet_MAT_Inst.Toilet_MAT_Inst" "None"))
  (bind _output_get (set `local.ToiletMaterial` _returnvalue))
  (`MaterialInstanceDynamic.SetVectorParameterValue` _output_get "Color" (`self.ToiletColor`))
  (if (`self.ColorSideOverride`)
    (`MaterialInstanceDynamic.SetScalarParameterValue` _output_get "OverrideColorSides" 1.0)
    (`PrimitiveComponent.SetMaterial` (`self.Toilet_FBX`) 0 (`local.ToiletMaterial`))
    (`PrimitiveComponent.SetMaterial` (`self.Toilet_Lid_FBX`) 0 (`local.ToiletMaterial`))))