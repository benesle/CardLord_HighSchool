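; Procedural wall actor that assembles a tiled wall from Width, Height and Thickness values.
; The construction script adds an instanced static mesh component per face, rotated and offset into place, then fills each with a grid of tile instances.
; It builds both main faces and the top, plus A and B end caps that are individually toggled or suppressed together by NoEndPieces.
; There is no bottom face or active runtime logic.
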(fn `UserConstructionScript`
  (locals (LocalTileSize :type Integer :default 100) (LocalWidthIndex :type Integer) (LocalHeightIndex :type Integer) (LocalSideThickness :type Integer :default 5) (LocalTotalHeight :type Integer) (LocalTotalWidth :type Integer) (LocalThicknessIndex :type Integer) (LocalTotalThickness :type Integer))
  (bind _returnvalue (`KismetMathLibrary.MakeTransform` (`KismetMathLibrary.MakeVector` (`KismetMathLibrary.Conv_IntToDouble` (* (`local.LocalHeightIndex`) (`local.LocalTileSize`))) (`KismetMathLibrary.Conv_IntToDouble` (* (`local.LocalWidthIndex`) (`local.LocalTileSize`))))))
  (bind _returnvalue_2 (`KismetMathLibrary.MakeTransform` (`KismetMathLibrary.MakeVector` 0.0 (`KismetMathLibrary.Conv_IntToDouble` (* (`local.LocalHeightIndex`) (`local.LocalTileSize`))) (`KismetMathLibrary.Conv_IntToDouble` (* (`local.LocalThicknessIndex`) (* (`local.LocalSideThickness`) -1)))) (`KismetMathLibrary.MakeRotator` 0.0)))
  (set `local.LocalTotalThickness` (* (`self.Thickness`) (`local.LocalSideThickness`)))
  (set `local.LocalTotalWidth` (* (`self.Width`) (`local.LocalTileSize`)))
  (set `local.LocalTotalHeight` (* (`self.Height`) (`local.LocalTileSize`)))
  (bind _returnvalue_3 (`AddComponent|NODE_AddInstancedStaticMeshComponent-2` :`RelativeTransform` (`KismetMathLibrary.MakeTransform` (0.0 0.0 0.0) (struct :`Pitch` 90.0))))
  (for _index (range (`self.Width`))
    (set `local.LocalWidthIndex` _index)
    (for _index_2 (range (`self.Height`))
      (set `local.LocalHeightIndex` _index_2)
      (`InstancedStaticMeshComponent.AddInstance` _returnvalue_3 _returnvalue)))
  (bind _returnvalue_4 (`AddComponent|NODE_AddInstancedStaticMeshComponent-4` :`RelativeTransform` (`KismetMathLibrary.MakeTransform` (`KismetMathLibrary.MakeVector` (`KismetMathLibrary.Conv_IntToDouble` (`local.LocalTotalThickness`)) (`KismetMathLibrary.Conv_IntToDouble` (`local.LocalTotalWidth`))) (struct :`Pitch` 90.0 :`Roll` 180.0))))
  (for _index_3 (range (`self.Width`))
    (set `local.LocalWidthIndex` _index_3)
    (for _index_4 (range (`self.Height`))
      (set `local.LocalHeightIndex` _index_4)
      (`InstancedStaticMeshComponent.AddInstance` _returnvalue_4 _returnvalue)))
  (bind _returnvalue_5 (`AddComponent|NODE_AddInstancedStaticMeshComponent-5` :`RelativeTransform` (`KismetMathLibrary.MakeTransform` (`KismetMathLibrary.MakeVector` (`KismetMathLibrary.Conv_IntToDouble` (`local.LocalTotalThickness`)) 0.0 (`KismetMathLibrary.Conv_IntToDouble` (`local.LocalTotalHeight`))) (`KismetMathLibrary.MakeRotator` 0.0 -90.0))))
  (for _index_5 (range (`self.Width`))
    (set `local.LocalWidthIndex` _index_5)
    (for _index_6 (range (`self.Thickness`))
      (set `local.LocalThicknessIndex` _index_6)
      (`InstancedStaticMeshComponent.AddInstance` _returnvalue_5 (`KismetMathLibrary.MakeTransform` (`KismetMathLibrary.MakeVector` 0.0 (`KismetMathLibrary.Conv_IntToDouble` (* (`local.LocalWidthIndex`) (`local.LocalTileSize`))) (`KismetMathLibrary.Conv_IntToDouble` (* (`local.LocalThicknessIndex`) (* (`local.LocalSideThickness`) -1)))) (`KismetMathLibrary.MakeRotator` 0.0)))))
  (if (not (`self.NoEndPieces`))
    (if (`self.A_Side`)
      (bind _returnvalue_6 (`AddComponent|NODE_AddInstancedStaticMeshComponent-8` :`RelativeTransform` (`KismetMathLibrary.MakeTransform` (`KismetMathLibrary.MakeVector` (`KismetMathLibrary.Conv_IntToDouble` (`local.LocalTotalThickness`))) (`KismetMathLibrary.MakeRotator` -90.0 0.0 90.0))))
      (for _index_7 (range (`self.Height`))
        (set `local.LocalHeightIndex` _index_7)
        (for _index_8 (range (`self.Thickness`))
          (set `local.LocalThicknessIndex` _index_8)
          (`InstancedStaticMeshComponent.AddInstance` _returnvalue_6 _returnvalue_2))))
    (if (`self.B_Side`)
      (bind _returnvalue_7 (`AddComponent|NODE_AddInstancedStaticMeshComponent-9` :`RelativeTransform` (`KismetMathLibrary.MakeTransform` (`KismetMathLibrary.MakeVector` (`KismetMathLibrary.Conv_IntToDouble` (`local.LocalTotalThickness`)) (`KismetMathLibrary.Conv_IntToDouble` (`local.LocalTotalWidth`)) (`KismetMathLibrary.Conv_IntToDouble` (`local.LocalTotalHeight`))) (`KismetMathLibrary.MakeRotator` 90.0 0.0 -90.0))))
      (for _index_9 (range (`self.Height`))
        (set `local.LocalHeightIndex` _index_9)
        (for _index_10 (range (`self.Thickness`))
          (set `local.LocalThicknessIndex` _index_10)
          (`InstancedStaticMeshComponent.AddInstance` _returnvalue_7 _returnvalue_2))))))