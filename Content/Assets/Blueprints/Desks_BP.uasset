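; Desks Blueprint that procedurally lays out a grid of tables with chairs, with no runtime logic.
; The construction script fills two instanced static mesh components from row, column and spacing variables, shifting chairs along Y by an offset.
; Each instance gets a random yaw within separate table and chair ranges, using streams seeded from SeedValue and grid indices so the layout is repeatable.
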(fn `UserConstructionScript`
  (locals (ColumnIndex :type Integer) (RowIndex :type Integer) (ChairOffset :type "Float (double-precision)" :default 25.0))
  (bind _chairrotationrange (`self.ChairRotationRange`))
  (bind _tablerotationrange (`self.TableRotationRange`))
  (bind _returnvalue (* (`local.ColumnIndex`) (`self.ColumnSpacing`)))
  (bind _returnvalue_2 (* (`local.RowIndex`) (`self.RowSpacing`)))
  (bind _returnvalue_3 (`AddComponent|NODE_AddInstancedStaticMeshComponent-0`))
  (for _index (range (`self.Columns`))
    (set `local.ColumnIndex` _index)
    (for _index_2 (range (`self.Rows`))
      (set `local.RowIndex` _index_2)
      (`InstancedStaticMeshComponent.AddInstance` _returnvalue_3 (`KismetMathLibrary.MakeTransform` (`KismetMathLibrary.MakeVector` _returnvalue_2 _returnvalue) (`KismetMathLibrary.MakeRotator` 0.0 0.0 (`KismetMathLibrary.RandomFloatInRangeFromStream` (* _tablerotationrange -1.0) _tablerotationrange (`KismetMathLibrary.MakeRandomStream` (* (`self.SeedValue`) (+ (`local.ColumnIndex`) (* (`local.RowIndex`) 23))))))))))
  (bind _returnvalue_4 (`AddComponent|NODE_AddInstancedStaticMeshComponent-1`))
  (for _index_3 (range (`self.Columns`))
    (set `local.ColumnIndex` _index_3)
    (for _index_4 (range (`self.Rows`))
      (set `local.RowIndex` _index_4)
      (`InstancedStaticMeshComponent.AddInstance` _returnvalue_4 (`KismetMathLibrary.MakeTransform` (`KismetMathLibrary.MakeVector` _returnvalue_2 (+ _returnvalue (`local.ChairOffset`))) (`KismetMathLibrary.MakeRotator` 0.0 0.0 (`KismetMathLibrary.RandomFloatInRangeFromStream` (* _chairrotationrange -1.0) _chairrotationrange (`KismetMathLibrary.MakeRandomStream` (* (+ (`self.SeedValue`) (* (`self.Rows`) (`self.Columns`))) (+ (`local.ColumnIndex`) (* (`local.RowIndex`) 13)))))))))))