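; Enemy Jock character blueprint that shows a sprite-textured enemy mesh playing a looping idle animation.
; On BeginPlay it creates a dynamic instance of the sprite material, applies it to the mesh and enables input from the first player controller.
; The L key flip-flops the material's sprite texture parameter between attack and idle textures, apparently as a test toggle.
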(event `self.ReceiveBeginPlay`
  (bind _enemy_jock_fbx (`self.Enemy_Jock_FBX`))
  (bind _returnvalue (`PrimitiveComponent.CreateDynamicMaterialInstance` _enemy_jock_fbx 0 "/Game/Character/Enemy/Materials/Enemy_Jock_SpriteMAT_Inst.Enemy_Jock_SpriteMAT_Inst" "None"))
  (`PrimitiveComponent.SetMaterial` _enemy_jock_fbx 0 _returnvalue)
  (`self.EnableInput` (`GameplayStatics.GetPlayerController` 0))
  (`SkeletalMeshComponent.PlayAnimation` (`self.Enemy_Jock_FBX`) "/Game/Character/Skeleton/Idle_ANIM.Idle_ANIM" true))

(event `Key|L`
  (params (Key :type "Key Structure"))
  (:`Pressed`
    (`/Engine/EditorBlueprintResources/StandardMacros.FlipFlop`
      (:`A`
        (`MaterialInstanceDynamic.SetTextureParameterValue` (stale `self.ReceiveBeginPlay` _returnvalue) "C_Sprite" "/Game/Character/Enemy/Textures/Enemy_Jock_Attack1.Enemy_Jock_Attack1"))
      (:`B`
        (`MaterialInstanceDynamic.SetTextureParameterValue` (stale `self.ReceiveBeginPlay` _returnvalue) "C_Sprite" "/Game/Character/Enemy/Textures/Enemy_Jock_Idle.Enemy_Jock_Idle")))))

(fn `UserConstructionScript`)