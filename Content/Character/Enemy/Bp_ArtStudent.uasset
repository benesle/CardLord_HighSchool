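; Art student enemy actor that records the current level as the flee map in the save game when any actor overlaps it.
; The overlap event loads slot A, writes the level name to FleeMap and saves back to that slot.
; An unconnected chain that would save player position, gold and inventory to a new save object never runs.
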(event `self.ReceiveActorBeginOverlap`
  (params (OtherActor :type "Actor Object Reference"))
  (bind _returnvalue (`GameplayStatics.LoadGameFromSlot` "A"))
  (bind _output_get (set `self.NewVar_1` _returnvalue))
  (bind _asnew_save_game (cast `/Game/UI/SaveGame/NewSaveGame` _output_get))
  (bind _returnvalue_2 (`GameplayStatics.GetCurrentLevelName` true))
  (set `/Game/UI/SaveGame/NewSaveGame.FleeMap` (`KismetStringLibrary.Conv_StringToName` _returnvalue_2) _asnew_save_game)
  (`GameplayStatics.SaveGameToSlot` _returnvalue "A"))

(fn `UserConstructionScript`)